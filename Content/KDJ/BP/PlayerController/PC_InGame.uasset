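; In-game player controller that provides keyboard shortcuts for lantern and MQTT message handling.
; BeginPlay finds the lantern and MQTT managers in the level, shows the cursor and sets Game and UI input.
; S injects an empty balloon "letter push" JSON message straight into the MQTT manager's OnMessage, simulating an incoming message.
; Delete clears all lanterns and Escape quits; a direct lantern spawn is left unconnected.
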(event `self.ReceiveBeginPlay`
  (bind _returnvalue (`GameplayStatics.GetActorOfClass` "/Game/KDJ/BP/BP_LanternManager.BP_LanternManager_C"))
  (set `self.LanternManager` _returnvalue)
  (bind _returnvalue_2 (`GameplayStatics.GetActorOfClass` "/Game/KDJ/BP/BP_MqttManager.BP_MqttManager_C"))
  (set `self.MqttManager` _returnvalue_2)
  (set `self.bShowMouseCursor` true)
  (`WidgetBlueprintLibrary.SetInputMode_GameAndUIEx` self null))

(event `Key|S`
  (params (Key :type "Key Structure"))
  (:`Pressed`
    (bind _outjsonstring (`|StructToJsonString` (make `/Game/KDJ/Data/S_EmptyBalloonDataMessage` (make `/Game/KDJ/Data/S_EmptyBalloonData` (make `/Game/KDJ/Data/S_EmptyBalloonDataHead` "content" "letter" "push") (struct)))))
    (`MqttManager.OnMessage` (`self.MqttManager`) "" _outjsonstring)))

(event `Key|Delete`
  (params (Key :type "Key Structure"))
  (:`Pressed`
    (`LanternManager.RemoveAllLantern` (`self.LanternManager`))
    (`KismetSystemLibrary.PrintString` "ALL LANTERNS DELETED")))

(event `Key|Escape`
  (params (Key :type "Key Structure"))
  (:`Pressed`
    (`KismetSystemLibrary.QuitGame` null "Quit")))

(fn `UserConstructionScript`)